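; Game instance for the battle royale game that tracks which front-end page is active and opens it.
; StartGame shows the splash widget with the mouse cursor and sets the page mode to Splash.
; SetMenuMode stores the new mode and calls OpenMenu, which shows a cached main menu widget or loads the lobby map.
; IsSplashPage reports whether the splash page is the current mode.
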(event Custom|StartGame
  ;[1 1 1] Start the Game - Splash
  (bind _returnvalue (UserInterface|CreateWidget "/Game/BattleRoyaleGame/Blueprints/HUD/BPW_Splash.BPW_Splash_C" (Game|GetPlayerController 0)))
  (UserInterface|Viewport|AddtoViewport _returnvalue 0)
  (Variables|/Script/Engine.PlayerController|SetbShowMouseCursor (Game|GetPlayerController 0) true)
  (Variables|Default|SetPageMode "NewEnumerator0"))

(event Custom|OpenMenu
  ;[1 1 1] Open Main Menu - Default Play
  (switch Utilities|FlowControl|Switch|SwitchonE_PageMode (Variables|Default|GetPageMode)
    (:NewEnumerator1
      (Variables|Default|GetMainMenu_Ref
        (:then
          _)
        (:else
          (bind _returnvalue (UserInterface|CreateWidget "/Game/BattleRoyaleGame/Blueprints/HUD/BPW_MainMenu.BPW_MainMenu_C" (Game|GetPlayerController 0)))
          (Variables|Default|SetMainMenu_Ref _returnvalue)))
      (UserInterface|Viewport|AddtoViewport (Variables|Default|GetMainMenu_Ref) 0))
    (:NewEnumerator6
      (Game|OpenLevel(byName) (Variables|Default|GetLobbyMap)))))

(event Custom|SetMenuMode
  (params (MenuMode :type E_PageMode%20Enum :default "NewEnumerator0"))
  ;[1 1 1] Open Main Menu - Default Play
  (Variables|Default|SetPageMode MenuMode)
  (CallFunction|OpenMenu))

(fn IsSplashPage
  (return (Utilities|Enum|Equal(Enum) (Variables|Default|GetPageMode) "NewEnumerator0")))
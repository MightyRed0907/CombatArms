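; Battle royale safe zone actor that moves and shrinks in steps, damaging players outside it; removed in deathmatch games.
; On game start the authority picks random next centers, taking speed, damage and pause from Steps.
; Tick moves the zone, deriving scale from distance travelled, while a one-second timer tracks overlaps and applies damage.
; Multicast events relay phases and minimap targets, remotes mirror shrink state, and admin events pause or resume it.
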(event Custom|GetNextPoint
  (bind (_x _y) (CallFunction|GetRandomLocation))
  (bind _finalshrinkvalue (Variables|Settings|GetFinalShrinkValue))
  ;[1 1 1] Get next point
  (Variables|Default|SetGoalScale (CallFunction|GetGoalScale))
  (bind _output_get (Variables|Default|SetFinalPoint (+ (Transformation|GetActorLocation) (Math|Vector|MakeVector _x _y 0.0))))
  (Variables|Default|SetLocDiff (- _output_get (Transformation|GetActorLocation)))
  (Variables|Default|SetInitScale (Transformation|GetWorldScale (Variables|Default|GetZoneMesh)))
  (if (CallFunction|SetupStep)
    (CallFunction|MCZonePaused _output_get (Variables|Default|GetGoalScale))
    (if (>= (Variables|Default|GetCurrentStep) 1)
      _
      (else
        (Variables|Default|SetGoalScale (Math|Vector|MakeVector _finalshrinkvalue _finalshrinkvalue (Variables|Settings|GetZoneZScale)))))
    (Utilities|Time|SetTimerbyEvent (delegate Custom|DelayedNextPoint) (Variables|Settings|GetPauseTime))))

(event Custom|DelayedNextPoint
  ;[1 1 1] Get next point
  (CallFunction|DoShrink (Variables|Default|GetFinalPoint) (Variables|Default|GetGoalScale) (Variables|Settings|GetShrinkInterpSpeed))
  (Variables|Default|SetChrink? true)
  (CallFunction|MCZoneMoving))

(event Custom|SetOverlapTimer
  (Utilities|Time|SetTimerbyEvent (delegate Custom|DamageTimer) 1.0 true))

(event Custom|AdminStopZone
  ;[1 1 1] Admin start and stop zone
  (Networking|SwitchHasAuthority
    (:Authority
      (if (Variables|Default|GetChrink?)
        (Variables|Default|SetChrink? false)
        (CallFunction|StopShrink (Transformation|GetWorldScale (Variables|Default|GetZoneMesh)) (Transformation|GetActorLocation) true)))))

(event Custom|AdminResumeZone
  ;[1 1 1] Admin start and stop zone
  (Networking|SwitchHasAuthority
    (:Authority
      (if (and (Variables|Default|GetZoneStarted?) (Variables|Default|GetFirstSetupDone))
        (Variables|Default|SetChrink? true)
        (CallFunction|MCZoneMoving)))))

(event Custom|AdminToggleStart
  ;[1 1 1] Admin start and stop zone
  (if (Variables|Default|GetChrink?)
    (CallFunction|AdminStopZone)
    (else
      (CallFunction|AdminResumeZone))))

(event Custom|StartZone
  (bind (_x _y) (CallFunction|GetRandomLocation))
  (bind _zonemesh (Variables|Default|GetZoneMesh))
  (bind _steps (Variables|Settings|GetSteps))
  (bind _returnvalue (Utilities|Array|Length _steps))
  (bind _returnvalue_2 (Transformation|GetWorldScale _zonemesh))
  (Rendering|SetActorHiddenInGame false)
  (Variables|Default|SetTotatlSteps _returnvalue)
  (bind _output_get (Variables|Default|SetCurrentStep _returnvalue))
  (if (> _output_get 0)
    (CallFunction|SetOverlapTimer)
    (Variables|Default|SetZoneStarted? true)
    (bind _output_get_2 (Variables|Default|SetFinalPoint (+ (Transformation|GetActorLocation) (Math|Vector|MakeVector _x _y 0.0))))
    (Variables|Default|SetLocDiff (- _output_get_2 (Transformation|GetActorLocation)))
    (Variables|Default|SetInitScale _returnvalue_2)
    (Variables|Default|SetStepScale (/ _returnvalue_2 (Variables|Default|GetTotatlSteps)))
    (bind _output_get_3 (Variables|Default|SetGoalScale (CallFunction|GetGoalScale)))
    (CallFunction|MCZoneStarted (Variables|Default|GetFinalPoint) _output_get_3)
    (Utilities|FlowControl|Delay (Variables|Settings|GetFirstDelay))
    (if (CallFunction|SetupStep)
      (CallFunction|DoShrink (Variables|Default|GetFinalPoint) (Variables|Default|GetGoalScale) (Variables|Settings|GetShrinkInterpSpeed))
      (Variables|Default|SetChrink? true)
      (CallFunction|MCZoneMoving)
      (Variables|Default|SetFirstSetupDone true))))

(event Custom|DamageTimer
  ;[1 1 1] Event for damage (every second)
  (CallFunction|HandlePlayersInside)
  (for _array_element (Variables|Default|GetPlayersOutside)
    (Utilities|IsValid _array_element
      (:Is%20Valid
        (bind _asbrcharacter (Utilities|Casting|CastToBRCharacter _array_element)
          (:then
            (Default|DamageTaken _asbrcharacter (Variables|Settings|GetDamagePerSec) (Variables|Settings|GetSourceName) 0 false))
          (:CastFailed
            (Game|Damage|ApplyDamage _array_element (Variables|Settings|GetDamagePerSec) 0 self "/Game/BattleRoyaleTemplateV2/4-World/WorldItems/DamageTypes/Zone.Zone_C")))))))

(event Custom|StopShrink
  (params (NewScale :type Vector) (NewLocation :type Vector) (AdminForced? :type Boolean))
  ;[1 1 1] Server events
  (Networking|SwitchHasAuthority
    (:Authority
      _)
    (:Remote
      (Variables|Default|SetChrink? false)
      (Transformation|SetWorldScale3D (Variables|Default|GetZoneMesh) NewScale)
      (Transformation|SetActorLocation NewLocation false false)))
  (if AdminForced?
    (Default|CallZoneSuspended)))

(event Custom|MC_ZoneStarted
  (params (NextPoint :type Vector) (TargetScale :type Vector))
  ;[1 1 1] Multicast events
  (Default|CallZoneStarted)
  (Rendering|SetActorHiddenInGame false)
  (Variables|Minimap|SetMinimap_NextLocation NextPoint)
  (Variables|Default|SetMinimap_TargetScale TargetScale)
  (Variables|Minimap|SetDrawNextPoint? true))

(event Custom|MC_ZonePaused
  (params (NextPoint :type Vector) (TargetScale :type Vector))
  ;[1 1 1] Multicast events
  (Default|CallZonePaused NextPoint)
  (Variables|Minimap|SetMinimap_NextLocation NextPoint)
  (Variables|Default|SetMinimap_TargetScale TargetScale)
  (Variables|Minimap|SetDrawNextPoint? true))

(event Custom|MC_ZoneEnded
  ;[1 1 1] Multicast events
  (Default|CallZoneEnded)
  (Variables|Minimap|SetDrawNextPoint? false))

(event Custom|MC_ZoneMoving
  ;[1 1 1] Multicast events
  (Default|CallZoneMoving))

(event Custom|DoShrink
  (params (FinalPoint :type Vector) (GoalScale :type Vector) (ShrinkInterpSpeed :type Float%20%28single-precision%29))
  ;[1 1 1] Server events
  (Networking|SwitchHasAuthority
    (:Remote
      (Variables|Settings|SetShrinkInterpSpeed ShrinkInterpSpeed)
      (bind _output_get (Variables|Default|SetFinalPoint FinalPoint))
      (Variables|Default|SetLocDiff (- _output_get (Transformation|GetActorLocation)))
      (Variables|Default|SetGoalScale GoalScale)
      (Variables|Default|SetInitScale (Transformation|GetWorldScale (Variables|Default|GetZoneMesh)))
      (Variables|Default|SetChrink? true))))

(event EventBeginPlay
  (Utilities|FlowControl|Sequence
    (:then_0
      (bind _asbr_game_instance (Utilities|Casting|CastToBR_GameInstance (Game|GetGameInstance)))
      (Variables|/Game/BattleRoyaleTemplateV2/0-MainBRClasses/BR_GameInstance.BR_GameInstance_C|SetZoneBP _asbr_game_instance self))
    (:then_1
      (Variables|/Script/Engine.PrimitiveComponent|SetbGenerateOverlapEvents (Variables|Default|GetZoneMesh) false)
      (Networking|SwitchHasAuthority
        (:Authority
          (Utilities|FlowControl|Sequence
            (:then_0
              (bind _asbr_game_instance_2 (Utilities|Casting|CastToBR_GameInstance (Game|GetGameInstance)))
              (if (Default|IsDeathMatchGame? _asbr_game_instance_2)
                (Actor|DestroyActor)))
            (:then_1
              (bind _asbr_game_state (Utilities|Casting|CastToBR_GameState (Game|GetGameState)))
              (EventDispatchers|BindEventtoGameStartedED _asbr_game_state (delegate Custom|StartZone))
              (Utilities|FlowControl|Delay 1.0 :!label _label)
              (Default|CallZonInitialized))))
        (:Remote
          (goto _label))))))

(event EventTick
  (params (DeltaSeconds :type Float%20%28single-precision%29))
  ;[1 1 1] Event tick for moving the zone
  (if (Variables|Default|GetChrink?)
    (Transformation|SetActorLocation (Math|Interpolation|VInterptoConstant (Transformation|GetActorLocation) (Variables|Default|GetFinalPoint) DeltaSeconds (Variables|Settings|GetShrinkInterpSpeed)) false false)
    (bind _output_get (Variables|Default|SetDeltaLoc (- 1.0 (/ (Math|Vector|VectorLength (- (Variables|Default|GetFinalPoint) (Transformation|GetActorLocation))) (Math|Vector|VectorLength (Variables|Default|GetLocDiff))))))
    (Transformation|SetWorldScale3D (Variables|Default|GetZoneMesh) (Math|Vector|Lerp(Vector) (Variables|Default|GetInitScale) (Variables|Default|GetGoalScale) _output_get))
    (if (<= (.x (Transformation|GetWorldScale (Variables|Default|GetZoneMesh))) (Variables|Settings|GetFinalShrinkValue))
      (Variables|Default|SetChrink? false)
      (Networking|SwitchHasAuthority
        (:Authority
          (CallFunction|MCZoneEnded)))
      (elif (== (Variables|Default|GetDeltaLoc) 1.0)
        (Variables|Default|SetChrink? false)
        (CallFunction|StopShrink (Transformation|GetWorldScale (Variables|Default|GetZoneMesh)) (Transformation|GetActorLocation) false)
        (CallFunction|GetNextPoint)))))

(fn ConstructionScript
  (bind _initialscale (Variables|Settings|GetInitialScale))
  (Transformation|SetWorldScale3D (Variables|Default|GetZoneMesh) (Math|Vector|MakeVector _initialscale _initialscale (Variables|Settings|GetZoneZScale))))

(fn GetActorRadius
  (bind _boxextent (Collision|GetActorBounds false false))
  (bind _returnvalue (/ (.x _boxextent) 2.0))
  (return _returnvalue (* _returnvalue -1.0)))

(fn GetZonePercent
  (return (/ (.x (Transformation|GetWorldScale (Variables|Default|GetZoneMesh))) (Variables|Settings|GetInitialScale))))

(fn GetRandomLocation
  (return (* (/ (.Radius (CallFunction|GetActorRadius)) 2.0) (CallFunction|GetRandomMultiplier)) (* (/ (.Radius (CallFunction|GetActorRadius)) 2.0) (CallFunction|GetRandomMultiplier))))

(fn GetRandomMultiplier
  (while (== (LocalVariables|GetResult) 0)
    (LocalVariables|SetResult (Math|Random|RandomIntegerinRange -1 1)))
  (return (Math|Conversions|ToFloat(Integer) (LocalVariables|GetResult))))

(fn GetGoalScale
  (bind _finalshrinkvalue (Variables|Settings|GetFinalShrinkValue))
  (bind _output_get (Variables|Default|SetCurrentStep (- (Variables|Default|GetCurrentStep) 1)))
  (if (> _output_get 0)
    (return (Math|Vector|MakeVector (.x (* (Variables|Default|GetStepScale) (Variables|Default|GetCurrentStep))) (.y (* (Variables|Default|GetStepScale) (Variables|Default|GetCurrentStep))) (Variables|Settings|GetZoneZScale)))
    (else
      (return (Math|Vector|MakeVector _finalshrinkvalue _finalshrinkvalue (Variables|Settings|GetZoneZScale))))))

(fn SetupStep
  (bind _steps (Variables|Settings|GetSteps))
  (bind _currentstep (Variables|Default|GetCurrentStep))
  (bind _returnvalue (Utilities|Array|Length _steps))
  (bind _returnvalue_2 (- _returnvalue _currentstep))
  (bind _returnvalue_3 (- _returnvalue_2 1))
  (bind _output (Utilities|Array|Get(acopy) _steps _returnvalue_3))
  (bind (_shrinkspeed _pausetime _damagepersec) (Utilities|Struct|BreakZoneStep _output))
  (if (and (>= _returnvalue_3 0) (< _returnvalue_3 _returnvalue))
    (Variables|Settings|SetShrinkInterpSpeed _shrinkspeed)
    (Variables|Settings|SetDamagePerSec _damagepersec)
    (Variables|Settings|SetPauseTime _pausetime)
    (return true)
    (else
      (return false))))

(fn HandlePlayersInside
  (bind _outactors (Collision|ComponentOverlapActors (Variables|Default|GetZoneMesh) (Transformation|GetActorTransform) (Utilities|Array|MakeArray "ObjectTypeQuery3") "/Script/Engine.Character"))
  (for _array_element _outactors
    (if (Utilities|Array|ContainsItem (Variables|Default|GetPlayersOutside) _array_element)
      (Utilities|Array|RemoveItem (Variables|Default|GetPlayersOutside) _array_element)
      (bind _asbrcharacter (Utilities|Casting|CastToBRCharacter _array_element)
        (:then
          (if (Variables|/Game/BattleRoyaleTemplateV2/2-BRCharacters/BRCharacter.BRCharacter_C|GetEnablePostProcessing? _asbrcharacter)
            (Default|PlayerinZoneStatus _asbrcharacter true)
            (Default|CLIENTPlayerinZoneStatus _asbrcharacter true)))
        (:CastFailed
          (Class|AIInterface|InZone(Message) _array_element self)))))
  (for _array_element_2 (Variables|Default|GetPlayerInCircle)
    (if (not (Utilities|Array|ContainsItem _outactors _array_element_2))
      (if (Utilities|IsValid _array_element_2)
        (Utilities|Array|Add (Variables|Default|GetPlayersOutside) _array_element_2)
        (bind _asbrcharacter_2 (Utilities|Casting|CastToBRCharacter _array_element_2)
          (:then
            (if (Variables|/Game/BattleRoyaleTemplateV2/2-BRCharacters/BRCharacter.BRCharacter_C|GetEnablePostProcessing? _asbrcharacter_2)
              (Default|PlayerinZoneStatus _asbrcharacter_2 false)
              (Default|CLIENTPlayerinZoneStatus _asbrcharacter_2 false)))
          (:CastFailed
            (Class|AIInterface|OutZone(Message) _array_element_2 self))))))
  (Variables|Default|SetPlayerInCircle _outactors))